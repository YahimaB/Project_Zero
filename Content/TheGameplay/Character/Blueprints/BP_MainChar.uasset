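; BP_MainChar is the player character Blueprint, handling camera orbit, camera-relative movement, jumping and Right Shift state tracking.
; Look input rotates CameraArm with clamped pitch and free yaw; CanTurn gates pitch but effectively not yaw, and EnableTurning sets it true on both press and release.
; Movement follows the arm's yaw and calls CancelMouseMovement when a mouse-move command is active, though that function is an empty stub.
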(event `InputAction|EnableTurning`
  (params (Key :type "Key Structure"))
  (:`Pressed`
    (set `self.CanTurn?` true))
  (:`Released`
    (set `self.CanTurn?` true)))

(event `InputAxis|LookUp`
  (params (AxisValue :type "Float (single-precision)"))
  ;[1 1 1] Camera UpDown Movement
  (if (and (`self.CanTurn?`) (!= AxisValue 0.0))
    (`SceneComponent.K2_SetRelativeRotation` (`self.CameraArm`) (`KismetMathLibrary.MakeRotator` (.roll (.rotation (`SceneComponent.GetRelativeTransform` (`self.CameraArm`)))) (`KismetMathLibrary.FClamp` (+ (.pitch (.rotation (`SceneComponent.GetRelativeTransform` (`self.CameraArm`)))) (* AxisValue 1.5)) -40.0 0.0) (.yaw (.rotation (`SceneComponent.GetRelativeTransform` (`self.CameraArm`))))) false false)))

(event `InputAxis|TurnRate`
  (params (AxisValue :type "Float (single-precision)"))
  ;[1 1 1] Camera LeftRight Movement
  (bind _returnvalue (+ AxisValue (stale `InputAxis|Turn` AxisValue)))
  (if (or (!= 0.0 AxisValue) (and (!= _returnvalue 0.0) (`self.CanTurn?`))) :!label _label
    (`SceneComponent.K2_SetRelativeRotation` (`self.CameraArm`) (`KismetMathLibrary.MakeRotator` (.roll (.rotation (`SceneComponent.GetRelativeTransform` (`self.CameraArm`)))) (.pitch (.rotation (`SceneComponent.GetRelativeTransform` (`self.CameraArm`)))) (+ (.yaw (.rotation (`SceneComponent.GetRelativeTransform` (`self.CameraArm`)))) (* _returnvalue 2.0))) false false)))

(event `InputAxis|Turn`
  (params (AxisValue :type "Float (single-precision)"))
  ;[1 1 1] Camera LeftRight Movement
  (goto _label))

(event `InputAxis|MoveForward`
  (params (AxisValue :type "Float (single-precision)"))
  ;[1 1 1] Button ForwardBack Movement
  (if (!= AxisValue 0.0)
    (if (`self.HasMouseMovementCommand?`)
      (`self.CancelMouseMovement`))
    (`self.AddMovementInput` (`KismetMathLibrary.GetForwardVector` (`KismetMathLibrary.MakeRotator` 0.0 0.0 (.yaw (.rotation (`SceneComponent.GetRelativeTransform` (`self.CameraArm`)))))) AxisValue)))

(event `InputAxis|MoveRight`
  (params (AxisValue :type "Float (single-precision)"))
  ;[1 1 1] Button RightLeft Movement
  (if (!= AxisValue 0.0)
    (if (`self.HasMouseMovementCommand?`)
      (`self.CancelMouseMovement`))
    (`self.AddMovementInput` (`KismetMathLibrary.GetRightVector` (`KismetMathLibrary.MakeRotator` 0.0 0.0 (.yaw (.rotation (`SceneComponent.GetRelativeTransform` (`self.CameraArm`)))))) AxisValue)))

(event `InputAction|Jump` :overrideparent false
  (params (Key :type "Key Structure"))
  ;[1 1 1] Button Jump
  (:`Pressed`
    (`self.Jump`))
  (:`Released`
    (`self.StopJumping`)))

(event `Key|RightShift`
  (params (Key :type "Key Structure"))
  ;[1 1 1] Button Right Shift
  (:`Pressed`
    (set `self.IsRightShifDown?` true))
  (:`Released`
    (set `self.IsRightShifDown?` false)))

(fn `CancelMouseMovement`)

(fn `UserConstructionScript`)