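; BP_ItemActor is a collectable world item that the player can pick up into their inventory.
; Its sphere collider registers and unregisters the item in the X_PlayerController's OverlappingItems list as the BP_MainChar enters or leaves range.
; On Interact, it calls the controller's AddItem, then destroys itself if everything fit or keeps the leftover as its new Amount.
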(event `self.SphereCollider.OnComponentBeginOverlap`
  (params (OverlappedComponent :type "PrimitiveComponent Object Reference") (OtherActor :type "Actor Object Reference") (OtherComp :type "PrimitiveComponent Object Reference") (OtherBodyIndex :type Integer) (bFromSweep :type Boolean) (SweepResult :type "HitResult Structure (by ref)"))
  (bind _asbp_main_char (cast `/Game/TheGameplay/Character/Blueprints/BP_MainChar` OtherActor)
    (:`then`
      (bind _asx_player_controller (cast `/Game/TheGameplay/Character/X_PlayerController` (`Pawn.GetController` _asbp_main_char))
        (:`then`
          (`KismetArrayLibrary.Array_Add` (`/Game/TheGameplay/Character/X_PlayerController.OverlappingItems` _asx_player_controller) self))
        (:`CastFailed`
          (`KismetSystemLibrary.PrintString` "Item Cast Fail: PC" true true (struct :`R` 1.0 :`A` 1.0) 10.0))))
    (:`CastFailed`
      (`KismetSystemLibrary.PrintString` "Item Cast Fail2: Char" true true (struct :`R` 1.0 :`A` 1.0) 10.0))))

(event `self.SphereCollider.OnComponentEndOverlap`
  (params (OverlappedComponent :type "PrimitiveComponent Object Reference") (OtherActor :type "Actor Object Reference") (OtherComp :type "PrimitiveComponent Object Reference") (OtherBodyIndex :type Integer))
  (bind _asbp_main_char (cast `/Game/TheGameplay/Character/Blueprints/BP_MainChar` OtherActor)
    (:`then`
      (bind _asx_player_controller (cast `/Game/TheGameplay/Character/X_PlayerController` (`Pawn.GetController` _asbp_main_char))
        (:`then`
          (`KismetArrayLibrary.Array_RemoveItem` (`/Game/TheGameplay/Character/X_PlayerController.OverlappingItems` _asx_player_controller) self))
        (:`CastFailed`
          (`KismetSystemLibrary.PrintString` "Item Cast Fail: PC" true true (struct :`R` 1.0 :`A` 1.0) 10.0))))
    (:`CastFailed`
      (`KismetSystemLibrary.PrintString` "Item Cast Fail1: Char" true true (struct :`R` 1.0 :`A` 1.0) 10.0))))

(event `/Game/TheGameplay/Items/Collectable/Inter_Item.Interact`
  (params (PlayerControllerRef :type "/Game/TheGameplay/Character/X_PlayerController Object Reference"))
  (`/Game/TheGameplay/Character/X_PlayerController.AddItem` PlayerControllerRef (`self.ItemNameToAdd`) (`self.Amount`))
  (`self.LiveOrDie` (`/Game/TheGameplay/Character/X_PlayerController.AddItemSuccess?` PlayerControllerRef) (`/Game/TheGameplay/Character/X_PlayerController.AddItemRest` PlayerControllerRef)))

(event `LiveOrDie`
  (params (`Success?` :type Boolean) (Rest :type Integer))
  (if `Success?`
    (if (== 0 Rest)
      (`self.K2_DestroyActor`)
      (else
        (set `self.Amount` Rest)))))

(fn `UserConstructionScript`)